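; BP_Box is a physics box that can be pulled toward a given location and thrown.
; Attract disables Box collision, enables physics on Cube, aims the NSBeam Niagara effect at the location and runs a timeline that applies an inward radial force.
; Throw turns off the beam, stops the timeline and, after a short delay, applies a stronger outward radial force from its supplied location.
; Both forces act as mass-independent acceleration changes with constant falloff.
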(event Custom|Attract
  (params (Location :type Vector))
  (bind _ns_beam (Variables|Default|GetNS_Beam))
  (bind _cube (Variables|Default|GetCube))
  (Collision|SetCollisionEnabled (Variables|Default|GetBox) "NoCollision")
  (Physics|SetSimulatePhysics (Variables|Default|GetCube) true)
  (Components|Activation|SetActive _ns_beam true true)
  (Effects|Components|ParticleSystem|SetVectorParameter _ns_beam "Location" Location)
  (Collision|SetCollisionEnabled _cube "QueryAndPhysics")
  (Timeline|Attract%20Timeline PlayFromStart
    (:NewTrack_0
      (Physics|AddRadialForce _cube Location 4e+03 -2e+04 "RIF_Constant" true))))

(event Custom|Throw
  (params (Location :type Vector))
  (Components|Activation|Deactivate (Variables|Default|GetNS_Beam))
  (Utilities|FlowControl|Sequence
    (:then_0
      (Timeline|Attract%20Timeline Stop
        (:NewTrack_0
          (Physics|AddRadialForce (Variables|Default|GetCube) (stale Custom|Attract Location) 4e+03 -2e+04 "RIF_Constant" true))))
    (:then_1
      (Utilities|FlowControl|Delay 0.2)
      (Physics|AddRadialForce (Variables|Default|GetCube) Location 4e+03 2e+05 "RIF_Constant" true))))

(fn ConstructionScript)